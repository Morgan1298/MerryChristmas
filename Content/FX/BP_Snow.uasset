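; BP_Snow is an effect actor that periodically randomizes the wind on its Niagara system, presumably falling snow.
; On BeginPlay it starts ChangeWind, which sets the User.WindPower parameter to a random positive or negative value and gives the actor a random yaw.
; The event prints a debug string, waits a random delay of several seconds, then calls itself, looping without Tick.
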(event Custom|ChangeWind
  (Niagara|SetNiagaraVariable(Float) (Variables|Default|GetNiagara) "User.WindPower" (Math|Random|RandomFloatinRange -3e+01 3e+01))
  (Transformation|SetActorRotation (Math|Rotator|MakeRotator 0.0 0.0 (Math|Random|RandomFloatinRange 0.0 3.6e+02)))
  (Development|PrintString "ChangingWind")
  (Utilities|FlowControl|Delay (Math|Random|RandomFloatinRange 5.0 2e+01))
  (CallFunction|ChangeWind))

(event EventBeginPlay
  (CallFunction|ChangeWind))

(event Collision|EventActorBeginOverlap
  (params (OtherActor :type Actor%20Object%20Reference)))

(event EventTick
  (params (DeltaSeconds :type Float%20%28single-precision%29)))

(fn ConstructionScript)